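; Followspot fixture Blueprint that swivels to track a target actor with its spotlight while Following is enabled.
; Each Tick, FollowSpot derives a look-at rotation from the base and eases the yoke's yaw and two body pivots' yaw and pitch toward it at FollowSpeed.
; The pivots use a fixed pitch offset, inverted on the second.
; A separate LightFade function, not called here, adjusts IES brightness from an accumulated value.
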(event EventTick
  (params (DeltaSeconds :type Float%20%28single-precision%29))
  (CallFunction|FollowSpot (Variables|AmIafollowspot?|GetFollowing?)))

(fn ConstructionScript)

(fn FollowSpot
  (params (Following? :type Boolean))
  (bind _target_for_light (Variables|AmIafollowspot?|GetTarget_for_Light))
  (bind _base (Variables|Default|GetBase))
  (bind _returnvalue (Transformation|GetActorLocation _target_for_light))
  (bind _returnvalue_2 (Transformation|GetWorldLocation _base))
  (bind _returnvalue_3 (Math|Rotator|FindLookatRotation _returnvalue_2 _returnvalue))
  (bind _returnvalue_4 (+ (.pitch _returnvalue_3) 8.0))
  ;[0.123 0 1] Follow the target and look correct while doing it
  (if Following?
    ;;[1 1 1] Yoke rotation
    (Transformation|SetWorldRotation (Variables|Default|GetYoke%20rotate) (Math|Interpolation|RInterpTo (Transformation|GetWorldRotation (Variables|Default|GetYoke%20rotate)) (Math|Rotator|MakeRotator 0.0 0.0 (.yaw _returnvalue_3)) (Utilities|Time|GetWorldDeltaSeconds) (Variables|AmIAFollowSpot?|GetFollow%20Speed)) false false)
    ;;[1 1 1] Spotlight Focus
    (Transformation|SetWorldRotation (Variables|Default|GetBodyRotate) (Math|Interpolation|RInterpTo (Transformation|GetWorldRotation (Variables|Default|GetBodyRotate)) (Math|Rotator|MakeRotator 0.0 _returnvalue_4 (.yaw _returnvalue_3)) (Utilities|Time|GetWorldDeltaSeconds) (Variables|AmIAFollowSpot?|GetFollow%20Speed)) false false)
    ;;[1 1 1] Body tilt
    (Transformation|SetWorldRotation (Variables|Default|GetBodyRotate2) (Math|Interpolation|RInterpTo (Transformation|GetWorldRotation (Variables|Default|GetBodyRotate2)) (Math|Rotator|MakeRotator 0.0 (* _returnvalue_4 -1.0) (.yaw _returnvalue_3)) (Utilities|Time|GetWorldDeltaSeconds) (Variables|AmIAFollowSpot?|GetFollow%20Speed)) false false)
    (else
      (return false))))

(fn LightFade
  (params (FadeAmount :type Float%20%28single-precision%29))
  (Variables|Default|SetForLoopIntensityInrecrease (+ (Variables|Default|GetForLoopIntensityInrecrease) FadeAmount))
  (Class|LightComponent|SetIESBrightnessScale (Variables|Default|GetSpotLight) (+ (Variables|Default|GetForLoopIntensityInrecrease) FadeAmount)))